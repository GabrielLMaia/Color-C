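; LevelControl is an actor that watches for the level being cleared of enemies.
; On BeginPlay it starts a looping timer that calls CheckFinish every few seconds to count actors tagged "Enemy".
; While enemies remain it prints MyGameMode's GameLevel; when none remain it calls PowerUp on MyGameMode.
; The timer is never cleared, so PowerUp repeats on each check that finds no enemies.
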(event `self.ReceiveBeginPlay`
  (`KismetSystemLibrary.K2_SetTimer` null "CheckFinish" 3.0 true))

(fn `CheckFinish`
  (bind _returnvalue (`GameplayStatics.GetGameMode`))
  (bind _outactors (`GameplayStatics.GetAllActorsWithTag` "Enemy"))
  (`/Engine/EditorBlueprintResources/StandardMacros.CompareInt` (`KismetArrayLibrary.Array_Length` _outactors)
    (:`>`
      (bind _asmy_game_mode (cast `/Game/BluePrint/Others/MyGameMode` _returnvalue))
      (`KismetSystemLibrary.PrintString` (`KismetStringLibrary.Conv_IntToString` (`/Game/BluePrint/Others/MyGameMode.game_level` _asmy_game_mode))))
    (:`==`
      (bind _asmy_game_mode_2 (cast `/Game/BluePrint/Others/MyGameMode` _returnvalue))
      (`/Game/BluePrint/Others/MyGameMode.PowerUp` _asmy_game_mode_2))))

(fn `UserConstructionScript`)