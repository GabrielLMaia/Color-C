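; BasicEnemy is a Paper2D enemy that gets a random color on spawn and takes damage from projectiles based on color match.
; Each Tick moves it along Z at Speed, with a timeline driving sideways movement.
; On overlap it explodes the projectile and loses player Damage divided by the squared summed RGB difference, so closer colors hit harder.
; At zero HP or below it is destroyed and adds PointValue to the player's Points.
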(event `self.ReceiveBeginPlay`
  ;[1 1 1] Setting initial color
  (`PrimitiveComponent.CreateDynamicMaterialInstance` (`self.PaperFlipbook`) 0 null)
  (bind _asmy_game_mode (cast `/Game/BluePrint/Others/MyGameMode` (`GameplayStatics.GetGameMode`)))
  (bind _output_get (set `self.min_color` (`/Game/BluePrint/Others/MyGameMode.min_color` _asmy_game_mode)))
  (bind _output_get_2 (set `self.Color` (`KismetMathLibrary.MakeVector` (`KismetMathLibrary.RandomFloatInRange` _output_get 1.0) (`KismetMathLibrary.RandomFloatInRange` _output_get 1.0) (`KismetMathLibrary.RandomFloatInRange` _output_get 1.0))))
  (`KismetSystemLibrary.PrintString` (`KismetStringLibrary.Conv_VectorToString` _output_get_2) true true (struct :`G` 0.66 :`B` 1.0 :`A` 1.0) 15.0)
  (`PaperFlipbookComponent.SetSpriteColor` (`self.PaperFlipbook`) (`KismetMathLibrary.Conv_VectorToLinearColor` _output_get_2))
  (`KismetSystemLibrary.PrintString` (`KismetStringLibrary.Conv_ColorToString` (`PaperFlipbookComponent.SpriteColor` (`self.PaperFlipbook`))) true true (struct :`R` 1.0 :`B` 0.858323 :`A` 1.0) 15.0))

(event `self.ReceiveActorBeginOverlap`
  (params (OtherActor :type "Actor Object Reference"))
  ;[1 1 1] Taking Damage
  (bind _asprojectile (cast `/Game/BluePrint/Player/Projectile` OtherActor))
  (bind (_returnvalue_x _returnvalue_y _returnvalue_z) (`KismetMathLibrary.BreakVector` (- (`self.Color`) (`/Game/BluePrint/Player/Projectile.color` _asprojectile))))
  (bind _newparam1 (`self.Damage Calculation` (+ (`KismetMathLibrary.Abs` _returnvalue_x) (`KismetMathLibrary.Abs` _returnvalue_y) (`KismetMathLibrary.Abs` _returnvalue_z))))
  (`/Game/BluePrint/Player/Projectile.Explode` _asprojectile _returnvalue_x _returnvalue_y _returnvalue_z)
  (bind _output_get (set `self.hp` (- (`self.hp`) _newparam1)))
  (`/Engine/EditorBlueprintResources/StandardMacros.CompareFloat` _output_get
    (:`==`
      _)
    (:`<`
      _))
  (`self.K2_DestroyActor`)
  (`self.Add Points To Pawn`))

(event `self.ReceiveTick`
  (params (DeltaSeconds :type "Float (single-precision)"))
  (bind (_direction _moviment) (`Timeline|Timeline_0`)
    (:`Update`
      (`self.K2_AddActorWorldOffset` (`KismetMathLibrary.MakeVector` (* _moviment (`self.side_speed`)) 0.0 (* DeltaSeconds (`self.speed`)))))))

(fn `Add Points To Pawn`
  (bind _asmain_character (cast `/Game/BluePrint/Player/MainCharacter` (`GameplayStatics.GetPlayerPawn` 0)))
  (set `/Game/BluePrint/Player/MainCharacter.points` (+ (`/Game/BluePrint/Player/MainCharacter.points` _asmain_character) (`self.point_value`)) _asmain_character))

(fn `Damage Calculation`
  (params (color_point :type "Float (double-precision)"))
  (returns (NewParam1 :type "Float (double-precision)"))
  (bind _asmain_character (cast `/Game/BluePrint/Player/MainCharacter` (`GameplayStatics.GetPlayerPawn` 0)))
  (bind _returnvalue (/ (`/Game/BluePrint/Player/MainCharacter.damage` _asmain_character) (* color_point color_point)))
  (`KismetSystemLibrary.PrintString` (`KismetStringLibrary.Conv_DoubleToString` _returnvalue) true true (struct :`R` 1.0 :`G` 0.98702 :`B` 0.976708 :`A` 1.0))
  (return _returnvalue))

(fn `UserConstructionScript`)