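; Boss enemy that cycles the color of its current sprite, starting with Dragon, after tinting Dragon, Circle and Rhombus red, green and blue.
; A looping timer keeps the Fixed channel constant and shifts the other two by random steps picked at BeginPlay.
; Each step is adjusted when its channel leaves the 0–1 range or reaches a limit.
; Every timer update also copies the player character's colors onto the Inner sprite.
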(event `self.ReceiveBeginPlay`
  (bind _max_var (`self.max_var`))
  (bind _min_var (`self.min_var`))
  (bind _asmy_game_mode (cast `/Game/BluePrint/Others/MyGameMode` (`GameplayStatics.GetGameMode`)))
  (bind _min_color (`/Game/BluePrint/Others/MyGameMode.min_color` _asmy_game_mode))
  (set `self.Color` (`|MakeArray` 1.0 _min_color _min_color))
  (`PaperFlipbookComponent.SetSpriteColor` (`self.Dragon`) (make `LinearColor` 1.0 _min_color _min_color 1.0))
  (`PaperFlipbookComponent.SetSpriteColor` (`self.Circle`) (make `LinearColor` _min_color 1.0 _min_color 1.0))
  (`PaperFlipbookComponent.SetSpriteColor` (`self.Rhombus`) (make `LinearColor` _min_color _min_color 1.0 1.0))
  (set `self.Atual` (`self.Dragon`))
  (set `self.randomC1` (`KismetMathLibrary.RandomFloatInRange` _min_var _max_var))
  (set `self.randomC2` (`KismetMathLibrary.RandomFloatInRange` _min_var _max_var))
  (`KismetSystemLibrary.K2_SetTimer` null "BossColorChange" 0.1 true))

(event `self.ReceiveTick`
  (params (DeltaSeconds :type "Float (single-precision)")))

(fn `BossColorChange`
  (bind _fixed (`self.fixed`))
  (bind _color (`self.Color`))
  (bind _output (`|GetArrayItem` (`self.Color`) (mod (+ _fixed 2) 3)))
  (bind _output_2 (`|GetArrayItem` (`self.Color`) (mod (+ _fixed 1) 3)))
  (`/Engine/EditorBlueprintResources/StandardMacros.CompareFloat` _output_2 1.0
    (:`>`
      (`/Engine/EditorBlueprintResources/StandardMacros.NegateFloat` (`self.randomC1`) :!label _label
        (:`  `
          _)))
    (:`==`
      (goto _label))
    (:`<`
      (`/Engine/EditorBlueprintResources/StandardMacros.CompareFloat` _output_2
        (:`>`
          _)
        (:`==`
          (goto _label))
        (:`<`
          (goto _label)))))
  (`/Engine/EditorBlueprintResources/StandardMacros.CompareFloat` _output 1.0
    (:`>`
      (`/Engine/EditorBlueprintResources/StandardMacros.NegateFloat` (`self.randomC2`) :!label _label_2
        (:`  `
          _)))
    (:`==`
      (goto _label_2))
    (:`<`
      (`/Engine/EditorBlueprintResources/StandardMacros.CompareFloat` _output
        (:`>`
          _)
        (:`==`
          (goto _label_2))
        (:`<`
          (goto _label_2)))))
  (`self.IncrementColor`)
  (`PaperFlipbookComponent.SetSpriteColor` (`self.Atual`) (make `LinearColor` (`|GetArrayItem` _color) (`|GetArrayItem` _color 1) (`|GetArrayItem` _color 2) 1.0))
  (bind _asmain_character (cast `/Game/BluePrint/Player/MainCharacter` (`GameplayStatics.GetPlayerPawn` 0)))
  (bind _colors (`/Game/BluePrint/Player/MainCharacter.colors` _asmain_character))
  (`PaperFlipbookComponent.SetSpriteColor` (`self.Inner`) (make `LinearColor` (`|GetArrayItem` _colors) (`|GetArrayItem` _colors 1) (`|GetArrayItem` _colors 2) 1.0)))

(fn `IncrementColor`
  (bind _color (`self.Color`))
  (bind _returnvalue (mod (+ (`self.fixed`) 2) 3))
  (bind _returnvalue_2 (mod (+ (`self.fixed`) 1) 3))
  (`KismetArrayLibrary.Array_Set` _color _returnvalue_2 (+ (`|GetArrayItem` (`self.Color`) _returnvalue_2) (`self.randomC1`)))
  (`KismetArrayLibrary.Array_Set` _color _returnvalue (+ (`|GetArrayItem` (`self.Color`) _returnvalue) (`self.randomC2`))))

(fn `UserConstructionScript`)