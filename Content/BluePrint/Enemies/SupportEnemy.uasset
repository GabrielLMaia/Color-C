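; Support enemy actor that drifts along Z, tinted red, green or blue at random unless preset.
; Projectiles overlapping its Box1 area get that color channel set to full.
; Player bullets hitting Box explode and deal the player's damage divided by squared color distance, so closer colors hurt more; PlayerBullet2 kills instantly.
; At zero health or below it destroys itself and awards points to the player.
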(event `self.ReceiveBeginPlay`
  (bind _color (`self.color`))
  (if (== (`self.aux`) -1)
    (bind _output_get (set `self.aux` (`KismetMathLibrary.RandomInteger` 3))))
  (switch `int` _output_get
    (:`Default`
      (set `self.color` (1.0 0.1 0.1) :!label _label))
    (:`0`
      (goto _label))
    (:`1`
      (set `self.color` (0.1 1.0 0.1)))
    (:`2`
      (set `self.color` (0.1 0.1 1.0))))
  (`PaperFlipbookComponent.SetSpriteColor` (`self.Attack`) (`KismetMathLibrary.Conv_VectorToLinearColor` _color))
  (`PaperFlipbookComponent.SetSpriteColor` (`self.Body`) (`KismetMathLibrary.Conv_VectorToLinearColor` _color)))

(event `self.Box1.OnComponentBeginOverlap`
  (params (OverlappedComponent :type "PrimitiveComponent Object Reference") (OtherActor :type "Actor Object Reference") (OtherComp :type "PrimitiveComponent Object Reference") (OtherBodyIndex :type Integer) (bFromSweep :type Boolean) (SweepResult :type "HitResult Structure (by ref)"))
  (bind _asmy_projectile (cast `/Game/BluePrint/Player/MyProjectile` OtherActor))
  (switch `int` (`self.aux`)
    (:`0`
      (bind (_color_x _color_y _color_z) (`KismetMathLibrary.BreakVector` (`/Game/BluePrint/Player/MyProjectile.color` _asmy_projectile)))
      (`/Game/BluePrint/Player/MyProjectile.ChangeColor` _asmy_projectile (`|MakeArray` 1.0 _color_y _color_z)))
    (:`1`
      (`/Game/BluePrint/Player/MyProjectile.ChangeColor` _asmy_projectile (`|MakeArray` _color_x 1.0 _color_z)))
    (:`2`
      (`/Game/BluePrint/Player/MyProjectile.ChangeColor` _asmy_projectile (`|MakeArray` _color_x _color_y 1.0)))))

(event `self.Box.OnComponentBeginOverlap`
  (params (OverlappedComponent :type "PrimitiveComponent Object Reference") (OtherActor :type "Actor Object Reference") (OtherComp :type "PrimitiveComponent Object Reference") (OtherBodyIndex :type Integer) (bFromSweep :type Boolean) (SweepResult :type "HitResult Structure (by ref)"))
  (if (`self.ActorHasTag` OtherActor "PlayerBullet")
    (bind _asmy_projectile (cast `/Game/BluePrint/Player/MyProjectile` OtherActor))
    (bind (_returnvalue_x _returnvalue_y _returnvalue_z) (`KismetMathLibrary.BreakVector` (- (`self.Color`) (`/Game/BluePrint/Player/MyProjectile.color` _asmy_projectile))))
    (bind _newparam1 (`self.damageCalculation` (`KismetMathLibrary.VSize` (`KismetMathLibrary.MakeVector` _returnvalue_x _returnvalue_y _returnvalue_z))))
    (`/Game/BluePrint/Player/MyProjectile.Explode` _asmy_projectile _returnvalue_x _returnvalue_y _returnvalue_z)
    (bind _output_get (set `self.hp` (- (`self.hp`) _newparam1)))
    (`/Engine/EditorBlueprintResources/StandardMacros.CompareFloat` _output_get :!label _label_2
      (:`==`
        _)
      (:`<`
        _))
    (`self.K2_DestroyActor`)
    (`self.addPoints`)
    (elif (`self.ActorHasTag` OtherActor "PlayerBullet2")
      (set `self.hp` 0.0)
      (goto _label_2))))

(event `self.ReceiveTick`
  (params (DeltaSeconds :type "Float (single-precision)"))
  (`self.K2_AddActorWorldOffset` (`KismetMathLibrary.MakeVector` 0.0 0.0 (* DeltaSeconds (`self.speed`)))))

(fn `addPoints`
  (bind _asmain_character (cast `/Game/BluePrint/Player/MainCharacter` (`GameplayStatics.GetPlayerPawn` 0)))
  (set `/Game/BluePrint/Player/MainCharacter.points` (+ (`/Game/BluePrint/Player/MainCharacter.points` _asmain_character) (`self.Point Value`)) _asmain_character))

(fn `damageCalculation`
  (params (ColorPoint :type "Float (double-precision)"))
  (returns (NewParam1 :type "Float (double-precision)"))
  (bind _returnvalue (+ ColorPoint 1e-07))
  (bind _asmain_character (cast `/Game/BluePrint/Player/MainCharacter` (`GameplayStatics.GetPlayerPawn` 0)))
  (bind _returnvalue_2 (/ (`/Game/BluePrint/Player/MainCharacter.damage` _asmain_character) (* _returnvalue _returnvalue)))
  (`KismetSystemLibrary.PrintString` (`KismetStringLibrary.Conv_DoubleToString` _returnvalue_2) true true (struct :`R` 1.0 :`G` 0.98702 :`B` 0.976708 :`A` 1.0))
  (return _returnvalue_2))

(fn `UserConstructionScript`)