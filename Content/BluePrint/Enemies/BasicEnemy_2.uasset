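; Color-matching 2D flipbook enemy that spawns with a random RGB tint, bounded below by the game mode's MinColor.
; PlayerBullet hits deal the player's Damage divided by squared RGB distance, so closer colors hurt more, while PlayerBullet2 deals heavy fixed damage.
; When Hp runs out it destroys itself and adds PointValue to the player's points.
; Tick moves it along Z, with timeline-driven sideways motion for Pattern 0.
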(event `self.ReceiveBeginPlay`
  ;[1 1 1] Setting initial color
  (`PrimitiveComponent.CreateDynamicMaterialInstance` (`self.PaperFlipbook`) 0 null)
  (bind _asmy_game_mode (cast `/Game/BluePrint/Others/MyGameMode` (`GameplayStatics.GetGameMode`)))
  (bind _output_get (set `self.min_color` (`/Game/BluePrint/Others/MyGameMode.min_color` _asmy_game_mode)))
  (bind _output_get_2 (set `self.Color` (`KismetMathLibrary.MakeVector` (`KismetMathLibrary.RandomFloatInRange` _output_get 1.0) (`KismetMathLibrary.RandomFloatInRange` _output_get 1.0) (`KismetMathLibrary.RandomFloatInRange` _output_get 1.0))))
  (`PaperFlipbookComponent.SetSpriteColor` (`self.PaperFlipbook`) (`KismetMathLibrary.Conv_VectorToLinearColor` _output_get_2)))

(event `self.ReceiveActorBeginOverlap`
  (params (OtherActor :type "Actor Object Reference"))
  (bind _hp (`self.hp`))
  ;[1 1 1] Taking Damage
  (if (`self.ActorHasTag` OtherActor "PlayerBullet")
    (bind _asmy_projectile (cast `/Game/BluePrint/Player/MyProjectile` OtherActor))
    (bind (_returnvalue_x _returnvalue_y _returnvalue_z) (`KismetMathLibrary.BreakVector` (- (`self.Color`) (`/Game/BluePrint/Player/MyProjectile.color` _asmy_projectile))))
    (bind _newparam1 (`self.Damage Calculation` (`KismetMathLibrary.VSize` (`KismetMathLibrary.MakeVector` _returnvalue_x _returnvalue_y _returnvalue_z))))
    (`/Game/BluePrint/Player/MyProjectile.Explode` _asmy_projectile _returnvalue_x _returnvalue_y _returnvalue_z)
    (bind _output_get (set `self.hp` (- _hp _newparam1)))
    (`/Engine/EditorBlueprintResources/StandardMacros.CompareFloat` _output_get :!label _label
      (:`==`
        _)
      (:`<`
        _))
    (`self.K2_DestroyActor`)
    (`self.Add Points To Pawn`)
    (elif (`self.ActorHasTag` OtherActor "PlayerBullet2")
      (`self.K2_DestroyActor` OtherActor)
      (set `self.hp` (- _hp 2000.0))
      (goto _label))))

(event `self.ReceiveTick`
  (params (DeltaSeconds :type "Float (single-precision)"))
  (bind _returnvalue (* DeltaSeconds (`self.speed`)))
  (switch `int` (`self.pattern`)
    (:`0`
      (bind (_direction _x) (`Timeline|Timeline_0`)
        (:`Update`
          (`self.K2_AddActorWorldOffset` (`KismetMathLibrary.MakeVector` (* _x (`self.side_speed`)) 0.0 _returnvalue)))))
    (:`1`
      (`self.K2_AddActorWorldOffset` (`KismetMathLibrary.MakeVector` 0.0 0.0 _returnvalue)))))

(fn `Add Points To Pawn`
  (bind _asmain_character (cast `/Game/BluePrint/Player/MainCharacter` (`GameplayStatics.GetPlayerPawn` 0)))
  (set `/Game/BluePrint/Player/MainCharacter.points` (+ (`/Game/BluePrint/Player/MainCharacter.points` _asmain_character) (`self.point_value`)) _asmain_character))

(fn `Damage Calculation`
  (params (color_point :type "Float (double-precision)"))
  (returns (NewParam1 :type "Float (double-precision)"))
  (bind _returnvalue (+ color_point 1e-07))
  (bind _asmain_character (cast `/Game/BluePrint/Player/MainCharacter` (`GameplayStatics.GetPlayerPawn` 0)))
  (bind _returnvalue_2 (/ (`/Game/BluePrint/Player/MainCharacter.damage` _asmain_character) (* _returnvalue _returnvalue)))
  (`KismetSystemLibrary.PrintString` (`KismetStringLibrary.Conv_DoubleToString` _returnvalue_2) true true (struct :`R` 1.0 :`G` 0.98702 :`B` 0.976708 :`A` 1.0))
  (return _returnvalue_2))

(fn `MovimentPattern`
  (params (pattern :type Integer))
  (switch `int` pattern
    (:`0`
      (set `self.Timeline_0` null))))

(fn `UserConstructionScript`)