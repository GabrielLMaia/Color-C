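; Player character Blueprint for a 2D color-based shooter, moving on the XZ plane, collecting points and losing energy to enemies, bosses and bullets until death opens Level1.
; A looping timer blends held RGB inputs into the sprite color with passive decay.
; Holding Shot auto-fires projectiles in that color through a gate and fire-rate delays.
; Stats load from the GameInstance, and PowerUp mode lets one be upgraded before GameMode advances the level.
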(event `InputAction|PowerUp1`
  (params (Key :type "Key Structure"))
  ;[1 1 1] PowerUp Input
  (:`Pressed`
    (`self.PowerUp` 1)))

(event `InputAxis|Red`
  (params (AxisValue :type "Float (single-precision)"))
  ;[1 1 1] Color inputs
  (`KismetArrayLibrary.Array_Set` (`self.color_increment`) 0 AxisValue))

(event `InputAction|PowerUp2`
  (params (Key :type "Key Structure"))
  ;[1 1 1] PowerUp Input
  (:`Pressed`
    (`self.PowerUp` 2)))

(event `self.ReceiveActorBeginOverlap`
  (params (OtherActor :type "Actor Object Reference"))
  ;[1 1 1] Taking Damage
  (if (`self.ActorHasTag` OtherActor "Point")
    (`self.K2_DestroyActor` OtherActor)
    (`/Engine/EditorBlueprintResources/StandardMacros.IncrementInt` (`self.points`))
    (elif (`self.ActorHasTag` OtherActor "Enemy")
      (cast `/Game/BluePrint/Enemies/BasicEnemy` OtherActor
        (:`then`
          (bind _output_get (set `self.energy` (- (`self.energy`) 20) :!label _label)))
        (:`CastFailed`
          (cast `/Game/BluePrint/Enemies/SupportEnemy` OtherActor
            (:`then`
              (goto _label))
            (:`CastFailed`
              (cast `/Game/BluePrint/Enemies/Boss` OtherActor
                (:`then`
                  _)
                (:`CastFailed`
                  (bind _asboss_bullet_1 (cast `/Game/BluePrint/Enemies/BossBullet1` OtherActor)
                    (:`then`
                      (`self.K2_DestroyActor` _asboss_bullet_1))
                    (:`CastFailed`
                      (bind _asboss_bullet_2 (cast `/Game/BluePrint/Enemies/BossBullet2` OtherActor))
                      (`self.K2_DestroyActor` _asboss_bullet_2)
                      (goto _label)))))
              (set `self.energy` (- (`self.energy`) 100))))))
      (`/Engine/EditorBlueprintResources/StandardMacros.CompareInt` _output_get
        (:`==`
          _)
        (:`<`
          _))
      (`self.Death`))))

(event `InputAction|PowerUp3`
  (params (Key :type "Key Structure"))
  ;[1 1 1] PowerUp Input
  (:`Pressed`
    (`self.PowerUp` 3)))

(event `InputAxis|Green`
  (params (AxisValue :type "Float (single-precision)"))
  ;[1 1 1] Color inputs
  (`KismetArrayLibrary.Array_Set` (`self.color_increment`) 1 AxisValue))

(event `InputAxis|Blue`
  (params (AxisValue :type "Float (single-precision)"))
  ;[1 1 1] Color inputs
  (`KismetArrayLibrary.Array_Set` (`self.color_increment`) 2 AxisValue))

(event `InputAction|Color-`
  (params (Key :type "Key Structure"))
  ;[1 1 1] Color inputs
  (:`Pressed`
    (set `self.clear` true))
  (:`Released`
    (set `self.clear` false)))

(event `self.ReceiveBeginPlay`
  ;[1 1 1] Start
  (bind _asmy_game_instance (cast `/Game/BluePrint/Others/MyGameInstance` (`GameplayStatics.GetGameInstance`)))
  (set `self.damage` (`/Game/BluePrint/Others/MyGameInstance.damage` _asmy_game_instance))
  (set `self.fire_rate` (`/Game/BluePrint/Others/MyGameInstance.firerate` _asmy_game_instance))
  (bind _output_get (set `self.max_energy` (`/Game/BluePrint/Others/MyGameInstance.max_energy` _asmy_game_instance)))
  (set `self.energy` _output_get)
  (set `self.points` (`/Game/BluePrint/Others/MyGameInstance.score` _asmy_game_instance))
  (bind _asmy_game_mode (cast `/Game/BluePrint/Others/MyGameMode` (`GameplayStatics.GetGameMode`)))
  (`KismetSystemLibrary.K2_SetTimer` null "UpdateChange" 0.1 true)
  (set `self.min_color` (`/Game/BluePrint/Others/MyGameMode.min_color` _asmy_game_mode)))

(event `self.ReceiveTick`
  (params (DeltaSeconds :type "Float (single-precision)")))

(event `InputAxis|Right`
  (params (AxisValue :type "Float (single-precision)"))
  ;[1 1 1] Character movement
  (`/Engine/EditorBlueprintResources/StandardMacros.CompareFloat` AxisValue
    (:`>`
      (`self.K2_SetActorRotation` (`KismetMathLibrary.MakeRotator` 0.0 270.0)))
    (:`<`
      (`self.K2_SetActorRotation` (`KismetMathLibrary.MakeRotator` 0.0 90.0))))
  (`self.K2_AddActorWorldOffset` (`KismetMathLibrary.MakeVector` (* AxisValue (`self.speed_sides`))) true))

(event `InputAction|Shot`
  (params (Key :type "Key Structure"))
  (bind (_returnvalue_location _returnvalue_rotation) (`KismetMathLibrary.BreakTransform` (`SceneComponent.K2_GetComponentToWorld` (`self.Arrow`))))
  ;[1 1 1] Shot Logic
  (:`Pressed`
    (`/Engine/EditorBlueprintResources/StandardMacros.DoOnce` false :!label _label_2
      (:`Completed`
        (`|ExecutionSequence`
          (:`then_0`
            (goto _label_3 :!via `Open`))
          (:`then_1`
            (`/Engine/EditorBlueprintResources/StandardMacros.Gate` true :!label _label_3
              (:`Exit`
                (`|ExecutionSequence`
                  (:`then_0`
                    (bind _returnvalue (`|SpawnActorFromClass` "/Game/BluePrint/Player/MyProjectile.MyProjectile_C" (`KismetMathLibrary.MakeTransform` _returnvalue_location _returnvalue_rotation (4.0 4.0 4.0)) "Undefined" "OverrideRootScale" null null))
                    (`/Game/BluePrint/Player/MyProjectile.ChangeColor` _returnvalue (`self.colors`))
                    (`KismetSystemLibrary.Delay` (`self.fire_rate`))
                    (goto _label_2 :!via `Reset`))
                  (:`then_1`
                    (`KismetSystemLibrary.RetriggerableDelay` (`self.fire_rate`))
                    (goto _label_3))))))))))
  (:`Released`
    (goto _label_3 :!via `Close`)))

(event `InputAxis|Up`
  (params (AxisValue :type "Float (single-precision)"))
  ;[1 1 1] Character movement
  (`/Engine/EditorBlueprintResources/StandardMacros.CompareFloat` AxisValue
    (:`>`
      (`self.K2_SetActorRotation` (`KismetMathLibrary.MakeRotator` 0.0)))
    (:`<`
      (`self.K2_SetActorRotation` (`KismetMathLibrary.MakeRotator` 0.0 180.0))))
  (`self.K2_AddActorWorldOffset` (`KismetMathLibrary.MakeVector` 0.0 0.0 (* AxisValue (`self.speed_up_down`))) true))

(fn `Death`
  (`GameplayStatics.OpenLevel` "Level1"))

(fn `IncrementColor`
  (bind _colors (`self.colors`))
  (bind _min_color (`self.min_color`))
  (for (_array_element _array_index) (`self.color_increment`)
    (if (`self.clear`)
      (`KismetArrayLibrary.Array_Set` _colors _array_index _min_color)
      (else
        (`KismetArrayLibrary.Array_Set` _colors _array_index (`KismetMathLibrary.FMax` (`KismetMathLibrary.FMin` (- (+ (* (`self.increment`) _array_element) (`|GetArrayItem` _colors _array_index)) (`self.passive_decrement`)) 1.0) _min_color))))))

(fn `PowerUp`
  (params (PowerUpType :type Integer))
  (bind _asmy_game_mode (cast `/Game/BluePrint/Others/MyGameMode` (`GameplayStatics.GetGameMode`)))
  (if (`KismetStringLibrary.EqualEqual_StrStr` (`/Game/BluePrint/Others/MyGameMode.game_mode` _asmy_game_mode) "PowerUp")
    (switch `int` PowerUpType
      (:`1`
        (set `self.fire_rate` (/ (`self.fire_rate`) 2.0)))
      (:`2`
        (set `self.damage` (* (`self.damage`) 2.0)))
      (:`3`
        (set `self.max_energy` (* (`self.max_energy`) 2))))
    (`/Game/BluePrint/Others/MyGameMode.NextLevel` _asmy_game_mode)))

(fn `UpdateChange`
  (bind _colors (`self.colors`))
  (`self.IncrementColor`)
  (`PaperFlipbookComponent.SetSpriteColor` (`self.Sprite`) (make `LinearColor` (`|GetArrayItem` _colors) (`|GetArrayItem` _colors 1) (`|GetArrayItem` _colors 2) 1.0)))

(fn `UserConstructionScript`)