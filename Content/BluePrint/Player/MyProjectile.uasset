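; MyProjectile is a flipbook projectile that can be tinted to a given character color and explodes to show a color difference.
; ChangeColor applies the supplied RGB to the sprite.
; Explode picks the red, green or blue difference with the largest magnitude, tints the sprite that pure channel color and plays a non-looping Plus or Minus flipbook by its sign.
; It then stops movement and expires shortly after.
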(fn `ChangeColor`
  (params (char_color :type "Array of Float (double-precision)"))
  (bind _output_get (set `self.color` (`KismetMathLibrary.MakeVector` (`|GetArrayItem` char_color) (`|GetArrayItem` char_color 1) (`|GetArrayItem` char_color 2))))
  (`PaperFlipbookComponent.SetSpriteColor` (`self.projectile`) (`KismetMathLibrary.Conv_VectorToLinearColor` _output_get)))

(fn `Explode`
  (params (red_dif :type "Float (double-precision)") (green_dif :type "Float (double-precision)") (blue_dif :type "Float (double-precision)"))
  (bind _returnvalue (`KismetMathLibrary.Abs` green_dif))
  (bind _returnvalue_2 (`KismetMathLibrary.Abs` blue_dif))
  (bind _returnvalue_3 (`KismetMathLibrary.Abs` red_dif))
  (bind _projectile (`self.projectile`))
  (bind _projectile_2 (`self.projectile`))
  (`/Engine/EditorBlueprintResources/StandardMacros.CompareFloat` _returnvalue_3 _returnvalue
    (:`>`
      (`/Engine/EditorBlueprintResources/StandardMacros.CompareFloat` _returnvalue_3 _returnvalue_2 :!label _label
        (:`>`
          (set `self.aux` (1.0 0.0 0.0) :!label _label_2)
          (`/Engine/EditorBlueprintResources/StandardMacros.CompareFloat` red_dif
            (:`>`
              (`PaperFlipbookComponent.SetLooping` _projectile_2 false :!label _label_3)
              (`PaperFlipbookComponent.SetFlipbook` _projectile "/Game/Sprites/Others/Plus/plus.plus"))
            (:`==`
              (goto _label_3))
            (:`<`
              (`PaperFlipbookComponent.SetLooping` _projectile_2 false :!label _label_4)
              (`PaperFlipbookComponent.SetFlipbook` _projectile "/Game/Sprites/Others/Minus/minus.minus"))))
        (:`==`
          (goto _label_2))
        (:`<`
          (set `self.aux` (0.0 0.0 1.0) :!label _label_5)
          (`/Engine/EditorBlueprintResources/StandardMacros.CompareFloat` blue_dif
            (:`>`
              (goto _label_3))
            (:`==`
              (goto _label_3))
            (:`<`
              (goto _label_4))))))
    (:`==`
      (goto _label))
    (:`<`
      (`/Engine/EditorBlueprintResources/StandardMacros.CompareFloat` _returnvalue _returnvalue_2
        (:`>`
          _)
        (:`==`
          _)
        (:`<`
          (goto _label_5)))
      (set `self.aux` (0.0 1.0 0.0))
      (`/Engine/EditorBlueprintResources/StandardMacros.CompareFloat` green_dif
        (:`>`
          (goto _label_3))
        (:`==`
          (goto _label_3))
        (:`<`
          (goto _label_4)))))
  (`PaperFlipbookComponent.SetSpriteColor` (`self.projectile`) (`KismetMathLibrary.Conv_VectorToLinearColor` (`self.aux`)))
  (`MovementComponent.StopMovementImmediately` (`self.ProjectileMovement`))
  (`self.SetLifeSpan` 0.5))

(fn `UserConstructionScript`)