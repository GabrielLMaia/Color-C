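; Background star actor built on a Paper2D sprite that scrolls vertically along world Z.
; On BeginPlay it caches GameSpeed from MyGameMode and gives the sprite an opaque, random mid-range color tint.
; Tick offsets the actor by that speed scaled by delta time, so later changes to GameSpeed do not affect stars already spawned.
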(event `self.ReceiveBeginPlay`
  (bind _asmy_game_mode (cast `/Game/BluePrint/Others/MyGameMode` (`GameplayStatics.GetGameMode`)))
  (set `self.speed` (`/Game/BluePrint/Others/MyGameMode.game_speed` _asmy_game_mode))
  (`PaperSpriteComponent.SetSpriteColor` (`self.PaperSprite`) (make `LinearColor` (`KismetMathLibrary.RandomFloatInRange` 0.3 0.7) (`KismetMathLibrary.RandomFloatInRange` 0.3 0.7) (`KismetMathLibrary.RandomFloatInRange` 0.3 0.7) 1.0)))

(event `self.ReceiveTick`
  (params (DeltaSeconds :type "Float (single-precision)"))
  (`self.K2_AddActorWorldOffset` (`KismetMathLibrary.MakeVector` 0.0 0.0 (* DeltaSeconds (`self.speed`)))))

(fn `UserConstructionScript`)