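; MyGameMode is a game mode Blueprint that sets up the HUD and handles power-up state and level progression.
; On BeginPlay it creates the main game and level-up widgets for player 0 and adds both to the viewport.
; PowerUp switches a GameMode state variable to power-up.
; NextLevel restores the playing state, increments GameLevel and opens a map whose name is built from "Level" plus that number.
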(event `self.ReceiveBeginPlay`
  (bind _returnvalue (`GameplayStatics.GetPlayerController` 0))
  (bind _returnvalue_2 (`|CreateWidget` "/Game/Hud/MainGameHud.MainGameHud_C" _returnvalue))
  (`UserWidget.AddToViewport` _returnvalue_2 0)
  (bind _returnvalue_3 (`|CreateWidget` "/Game/Hud/LevelUpHud.LevelUpHud_C" _returnvalue))
  (`UserWidget.AddToViewport` _returnvalue_3 0))

(fn `NextLevel`
  (set `self.game_mode` "Playing")
  (bind _result (`/Engine/EditorBlueprintResources/StandardMacros.IncrementInt` (`self.game_level`))
    (:`  `
      (`GameplayStatics.OpenLevel` (`KismetStringLibrary.Conv_StringToName` (`KismetStringLibrary.BuildString_Int` "Level" "" _result)) false))))

(fn `PowerUp`
  (set `self.game_mode` "PowerUp"))

(fn `UserConstructionScript`)