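; Game instance that holds a snapshot of player stats and game progress.
; UpdateValues copies damage, fire rate, max energy and points from the player's MainCharacter pawn, storing points as Score.
; It then copies the current game level from MyGameMode, stopping early if either cast fails.
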(fn `Update Values`
  (bind _asmain_character (cast `/Game/BluePrint/Player/MainCharacter` (`GameplayStatics.GetPlayerPawn` 0)))
  (set `self.damage` (`/Game/BluePrint/Player/MainCharacter.damage` _asmain_character))
  (set `self.firerate` (`/Game/BluePrint/Player/MainCharacter.fire_rate` _asmain_character))
  (set `self.max_energy` (`/Game/BluePrint/Player/MainCharacter.max_energy` _asmain_character))
  (set `self.score` (`/Game/BluePrint/Player/MainCharacter.points` _asmain_character))
  (bind _asmy_game_mode (cast `/Game/BluePrint/Others/MyGameMode` (`GameplayStatics.GetGameMode`)))
  (set `self.level` (`/Game/BluePrint/Others/MyGameMode.game_level` _asmy_game_mode)))